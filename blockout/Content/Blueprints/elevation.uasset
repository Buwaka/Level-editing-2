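; Climb volume Blueprint that raises an overlapping actor while Jump is held.
; Overlap events track whether something is inside and store the last actor to enter.
; Each Tick, it sets player 0 to Flying and offsets the stored actor upward by ClimbSpeed, without sweep or delta-time scaling.
; Releasing Jump stops the climb and restores Walking, whether or not the player is inside.
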(event `self.ReceiveTick`
  (params (DeltaSeconds :type "Float (single-precision)"))
  (bind _actor (`self.Actor`))
  (if (and (`self.IsInside`) (`self.GoUpwards`))
    (`CharacterMovementComponent.SetMovementMode` (`Character.CharacterMovement` (`GameplayStatics.GetPlayerCharacter` 0)) "MOVE_Flying" 0)
    (bind (_sweephitresult _returnvalue) (`self.K2_SetActorLocation` _actor (+ (`self.K2_GetActorLocation` _actor) (`KismetMathLibrary.MakeVector` 0.0 0.0 (`self.climb speed`))) false false))))

(event `self.ReceiveActorEndOverlap`
  (params (OtherActor :type "Actor Object Reference"))
  (set `self.IsInside` false))

(event `self.ReceiveActorBeginOverlap`
  (params (OtherActor :type "Actor Object Reference"))
  (set `self.IsInside` true)
  (set `self.Actor` OtherActor))

(event `InputAction|Jump` :consume false
  (params (Key :type "Key Structure"))
  (:`Pressed`
    (set `self.GoUpwards` true))
  (:`Released`
    (set `self.GoUpwards` false)
    (`CharacterMovementComponent.SetMovementMode` (`Character.CharacterMovement` (`GameplayStatics.GetPlayerCharacter` 0)) "MOVE_Walking" 0)))

(fn `UserConstructionScript`)