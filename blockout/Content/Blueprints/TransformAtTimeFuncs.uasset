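; Blueprint function that looks up the transform recorded at a given timestamp in an array of timestamped transforms.
; It scans from the end of the array and returns the first transform whose timestamp is at or before the requested time, without interpolation.
; Later entries it passes are removed from the array, except index zero, whose transform is the fallback when nothing matches.
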(fn `Get_Transform_At_Timestamp`
  (params (Timestamp :type "Float (double-precision)") (Array :type "Array of /Game/Blueprints/TransformsAtTime Structure (by ref)"))
  (returns (Transform :type "Transform Structure"))
  (locals (last :type "Transform Structure"))
  (bind _output_get (set `local.last` (`.Transform_4_49B1F4F94DEDAAC500DC6ABC9CCF9606` (break `/Game/Blueprints/TransformsAtTime` (`|GetArrayItem` Array)))))
  (bind (_arrayindex _arrayelement) (`/Engine/EditorBlueprintResources/StandardMacros.ReverseForEachLoop` Array)
    (:`LoopBody`
      (bind (_transform _timestamp) (break `/Game/Blueprints/TransformsAtTime` _arrayelement))
      (if (<= _timestamp Timestamp)
        (return _transform)
        (elif (> _arrayindex 0)
          (`KismetArrayLibrary.Array_Remove` Array _arrayindex))))
    (:`Completed`
      (return _output_get))))