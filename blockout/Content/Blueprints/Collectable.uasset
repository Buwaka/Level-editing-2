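; Collectable actor that shows a Pickup widget while an actor overlaps it, with no collection logic in its graphs.
; BeginPlay creates the widget for the first player controller, adds it to the viewport and hides it.
; Begin and end overlap events toggle its visibility without checking which actor overlaps.
; The construction script sizes the Sphere component from the CollissionRadius variable.
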(event `self.ReceiveBeginPlay`
  (bind _returnvalue (`|CreateWidget` "/Game/Blueprints/pickup.pickup_C" (`GameplayStatics.GetPlayerController` 0)))
  (bind _output_get (set `self.pickup widget` _returnvalue))
  (`UserWidget.AddToViewport` _output_get 0)
  (`Widget.SetVisibility` _output_get "Hidden"))

(event `self.ReceiveActorBeginOverlap`
  (params (OtherActor :type "Actor Object Reference"))
  (`Widget.SetVisibility` (`self.pickup widget`) "Visible"))

(event `self.ReceiveActorEndOverlap`
  (params (OtherActor :type "Actor Object Reference"))
  (`Widget.SetVisibility` (`self.pickup widget`) "Hidden"))

(fn `UserConstructionScript`
  (`SphereComponent.SetSphereRadius` (`self.Sphere`) (`self.collission radius`) true))